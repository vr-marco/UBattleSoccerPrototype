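; Behavior tree task that makes a soccer bot pursue the actor stored in the PursuitActor blackboard key.
; It clips the target's location to the bot's action zone, flattens it to the bot's height and issues a simple move there.
; It also writes a behavior string naming the target as a player, soccer ball or other actor.
; It finishes as failed right after issuing the move, and as succeeded when no valid target exists.
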(event EventReceiveExecute
  (params (OwnerActor :type Actor%20Object%20Reference))
  (bind _array (Utilities|Array|MakeArray 0))
  (bind _blackboardkeyselector (Utilities|Struct|MakeBlackboardKeySelector _array "PursuitActor"))
  (bind _returnvalue (Class|BTFunctionLibrary|GetBlackboardValueasObject _blackboardkeyselector))
  ;[1 1 1] Cache values for easier reading
  (bind _assoccer_bot_controller (Utilities|Casting|CastToSoccerBotController OwnerActor))
  (Variables|Default|SetMySoccerBotControllerRef _assoccer_bot_controller)
  (bind _asmagic_battle_soccer_character (Utilities|Casting|CastToMagicBattleSoccerCharacter (Pawn|GetControlledPawn _assoccer_bot_controller)))
  (Variables|Default|SetMyCharacterRef _asmagic_battle_soccer_character)
  ;[1 1 1] Determine if we're pursuing anything
  (Utilities|IsValid _returnvalue
    (:Is%20Valid
      (bind _asactor (Utilities|Casting|CastToActor _returnvalue))
      (bind _behaviorstring (CallFunction|GetBehaviorString _asactor))
      (Variables|/Game/Blueprints/Pawns/SoccerBotController.SoccerBotController_C|SetCurrentBehaviorString (Variables|Default|GetMySoccerBotControllerRef) (Utilities|String|Append "Pursuing " _behaviorstring))
      ;[1 1 1] Cache the pursuit actor's location
      (Variables|Default|SetTargetLocation (Transformation|GetActorLocation _asactor))
      ;[1 1 1] Move to the actor
      (bind _returnvalue_2 (Class|MagicBattleSoccerAIController|CliptoActionZone (Variables|Default|GetMySoccerBotControllerRef) (Variables|Default|GetTargetLocation)))
      (AI|Navigation|SimpleMovetoLocation (Variables|Default|GetMySoccerBotControllerRef) (Math|Vector|MakeVector (.X (Math|Vector|BreakVector _returnvalue_2)) (.Y (Math|Vector|BreakVector _returnvalue_2)) (.Z (Math|Vector|BreakVector (Transformation|GetActorLocation (Variables|Default|GetMyCharacterRef))))))
      (AI|BehaviorTree|FinishExecute false))
    (:Is%20Not%20Valid
      (AI|BehaviorTree|FinishExecute true))))

(fn GetBehaviorString
  (params (Actor :type Actor%20Object%20Reference))
  (bind _asmagic_battle_soccer_character (Utilities|Casting|CastToMagicBattleSoccerCharacter Actor)
    (:then
      (bind _playerstate (Variables|/Script/Engine.Pawn|GetPlayerState _asmagic_battle_soccer_character)
        (:then
          (LocalVariables|SetActorName (PlayerState|GetPlayerName _playerstate)))
        (:else)))
    (:CastFailed
      (Utilities|Casting|CastToSoccerBall Actor
        (:then
          (LocalVariables|SetActorName "soccer ball"))
        (:CastFailed
          (LocalVariables|SetActorName "other actor")))))
  (return (LocalVariables|GetActorName)))